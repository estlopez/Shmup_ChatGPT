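; Player ship for a shooter that moves on the X/Z plane and stays confined to a ScrollBox volume.
; BeginPlay spawns a TriShotWeapon at WeaponPoint, attaches it, and switches the view to the first CameraController found in the level.
; Move offsets the Ship component without sweeping, and Tick clamps its world position to the box extents on all axes.
; Shoot start and stop events are forwarded to the current weapon.
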(event EventBeginPlay
  (CallFunction|WeaponEquip)
  (CallFunction|SetNewCameraTarget))

(event EventCanShoot
  (Default|CanShoot (Variables|Default|GetCurrentWeapon)))

(event EventStopShooting
  (Default|StopShooting (Variables|Default|GetCurrentWeapon)))

(event EventTick
  (params (DeltaSeconds :type Float%20%28single-precision%29))
  (bind _ship (Variables|Default|GetShip))
  (bind _scrollbox (Variables|Default|GetScrollBox))
  (bind _returnvalue (Transformation|GetWorldLocation _ship))
  (bind _returnvalue_2 (Transformation|GetWorldLocation _scrollbox))
  (bind _returnvalue_3 (Components|Box|GetScaledBoxExtent _scrollbox))
  (Transformation|SetWorldLocation _ship (Math|Vector|MakeVector (Math|Float|Clamp(Float) (.x _returnvalue) (- (.x _returnvalue_2) (.x _returnvalue_3)) (+ (.x _returnvalue_2) (.x _returnvalue_3))) (Math|Float|Clamp(Float) (.y _returnvalue) (- (.y _returnvalue_2) (.y _returnvalue_3)) (+ (.y _returnvalue_2) (.y _returnvalue_3))) (Math|Float|Clamp(Float) (.z _returnvalue) (- (.z _returnvalue_2) (.z _returnvalue_3)) (+ (.z _returnvalue_2) (.z _returnvalue_3)))) false false))

(fn ConstructionScript)

(fn WeaponEquip
  (bind _weapon_point (Variables|Default|GetWeapon_Point))
  (bind _returnvalue (Game|SpawnActorfromClass "/Game/Blueprints/AutoGenerated/TriShotWeapon.TriShotWeapon_C" (Transformation|GetWorldTransform _weapon_point) "Undefined" "MultiplyWithRoot" 0 0))
  (bind _output_get (Variables|Default|SetCurrentWeapon _returnvalue))
  (Transformation|AttachComponentToComponent _output_get _weapon_point "None" "SnapToTarget" "KeepRelative" "KeepRelative" true))

(fn Move
  (params (Z :type Float%20%28double-precision%29) (X :type Float%20%28double-precision%29))
  (Transformation|AddRelativeLocation (Variables|Default|GetShip) (Math|Vector|MakeVector X 0.0 Z) false false))

(fn SetNewCameraTarget
  (bind _outactors (Actor|GetAllActorsOfClass "/Game/Blueprints/AutoGenerated/CameraController.CameraController_C"))
  (Game|Player|SetViewTargetwithBlend (Pawn|GetLocalViewingPlayerController (Game|Player|GetPlayerPawn 0)) (Utilities|Array|Get(acopy) _outactors) 0.0 "VTBlend_Linear" 0.0 false))