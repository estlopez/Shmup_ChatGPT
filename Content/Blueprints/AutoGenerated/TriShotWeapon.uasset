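; Player weapon Blueprint that fires a three-projectile volley and auto-repeats while shooting is active.
; CanShoot fires immediately, then starts a looping half-second timer on Shoot; StopShooting clears that timer through its stored handle.
; Shoot spawns a PlayerProjectile at the world transform of each of the TopShot, MidShot and LowShot components.
; BeginPlay sets the WeaponType enum that identifies this weapon.
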(event EventBeginPlay
  (Variables|Default|SetWeaponType "NewEnumerator1"))

(event EventCanShoot
  (CallFunction|Shoot)
  (bind _returnvalue (Utilities|Time|SetTimerbyFunctionName 0 "Shoot" 0.5 true))
  (Variables|Default|SetShootTimerHandle _returnvalue))

(event EventStopShooting
  (Utilities|Time|ClearandInvalidateTimerbyHandle (Variables|Default|GetShootTimerHandle)))

(fn ConstructionScript
  (|CallParentFunction))

(fn Shoot
  (for _array_element (Utilities|Array|MakeArray (Variables|Default|GetTop_Shot) (Variables|Default|GetMid_Shot) (Variables|Default|GetLow_Shot))
    (Game|SpawnActorfromClass "/Game/Blueprints/AutoGenerated/PlayerProjectile.PlayerProjectile_C" (Transformation|GetWorldTransform _array_element) "Undefined" "MultiplyWithRoot" 0 0)))