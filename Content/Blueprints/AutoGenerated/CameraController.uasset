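; CameraController relays player input to the PlayerShip pawn, despite its name containing no camera logic.
; On BeginPlay it caches the ship and adds the Enhanced Input mapping context.
; Two move actions feed scaled axis values into the ship's Move call on separate axes.
; Fire press calls CanShoot after a BPI_Fire interface check, while release or cancel calls StopShooting without one.
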(event Input|EnhancedActionEvents|EnhancedInputActionINP_Move
  (params (ActionValue :type Vector%202D%20Structure) (ElapsedSeconds :type Float%20%28double-precision%29) (TriggeredSeconds :type Float%20%28double-precision%29) (InputAction :type Input%20Action%20Object%20Reference :default "/Game/Blueprints/Input/INP_Move.INP_Move"))
  (Default|Move (Variables|Default|GetPlayerRef) (* (.X (Math|Vector2D|BreakVector2D ActionValue)) 7.0) 0.0))

(event Input|EnhancedActionEvents|EnhancedInputActionINP_Fire
  (params (ActionValue :type Boolean) (ElapsedSeconds :type Float%20%28double-precision%29) (TriggeredSeconds :type Float%20%28double-precision%29) (InputAction :type Input%20Action%20Object%20Reference :default "/Game/Blueprints/Input/INP_Fire.INP_Fire"))
  (:Started
    (CallFunction|ShotFunction))
  (:Canceled
    (CallFunction|StopFiringFunction :!label _label))
  (:Completed
    (goto _label)))

(event Input|EnhancedActionEvents|EnhancedInputActionINP_Move_Fwd
  (params (ActionValue :type Vector%202D%20Structure) (ElapsedSeconds :type Float%20%28double-precision%29) (TriggeredSeconds :type Float%20%28double-precision%29) (InputAction :type Input%20Action%20Object%20Reference :default "/Game/Blueprints/Input/INP_Move_Fwd.INP_Move_Fwd"))
  (Default|Move (Variables|Default|GetPlayerRef) 0.0 (* (.X (Math|Vector2D|BreakVector2D ActionValue)) 7.0)))

(event EventBeginPlay
  (bind _returnvalue (Game|GetPlayerController 0))
  (bind _asplayer_ship (Utilities|Casting|CastToPlayerShip (Game|Player|GetPlayerPawn 0)))
  (Variables|Default|SetPlayerRef _asplayer_ship)
  (Utilities|IsValid _returnvalue
    (:Is%20Valid
      (Input|AddMappingContext (PlayerController|LocalPlayerSubsystems|GetEnhancedInputLocalPlayerSubsystem _returnvalue) "/Game/Blueprints/Input/CONTEXT_Input.CONTEXT_Input" 0 "(bIgnoreAllPressedKeysUntilRelease=True,bForceImmediately=False,bNotifyUserSettings=False)"))))

(fn ConstructionScript)

(fn ShotFunction
  (bind _playerref (Variables|Default|GetPlayerRef))
  (if (Utilities|DoesObjectImplementInterface _playerref "/Game/Blueprints/AutoGenerated/BPI_Fire.BPI_Fire_C")
    (Default|CanShoot _playerref)))

(fn StopFiringFunction
  (Default|StopShooting (Variables|Default|GetPlayerRef)))